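; Game mode for a Space Invaders-style game that sets the view to a level camera and spawns the alien (Alieno) grid on BeginPlay.
; A looping timer moves all aliens sideways, applying the offset once per alien checked, so step size scales with alien count.
; When an alien reaches either side limit, MovimentoBasso drops the formation, flips VadoADestra and restarts horizontal movement.
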(event Custom|MovimentoAlieno
  ;[0.15 0.15 0.15 0.5] Movimento Alieno
  (bind _outactors (Actor|GetAllActorsOfClass "/Game/Blueprints/Alieno.Alieno_C"))
  (for _array_element _outactors
    (if (Variables|Default|GetVado%20a%20destra?)
      (if (>= (.y (Transformation|GetWorldLocation (Variables|/Game/Blueprints/Alieno.Alieno_C|GetDefaultSceneRoot _array_element))) 7.9e+02)
        (Class|KismetSystemLibrary|PauseTimer 0 "MovimentoAlieno")
        (Utilities|Time|SetTimerbyFunctionName 0 "MovimentoBasso" 0.5 true)
        (else
          (Transformation|AddActorWorldOffset _outactors (Math|Vector|MakeVector 0.0 2.0 0.0))))
      (elif (<= (.y (Transformation|GetWorldLocation (Variables|/Game/Blueprints/Alieno.Alieno_C|GetDefaultSceneRoot _array_element))) -7.9e+02)
        (Class|KismetSystemLibrary|PauseTimer 0 "MovimentoAlieno")
        (Utilities|Time|SetTimerbyFunctionName 0 "MovimentoBasso" 0.5 true)
        (else
          (Transformation|AddActorWorldOffset _outactors (Math|Vector|MakeVector 0.0 -2.0 0.0)))))))

(event Custom|MovimentoBasso
  ;[0.15 0.15 0.15 0.5] Movimento Alieno
  (bind _outactors (Actor|GetAllActorsOfClass "/Game/Blueprints/Alieno.Alieno_C"))
  (Transformation|AddActorWorldOffset _outactors (Math|Vector|MakeVector 0.0 0.0 -6e+01))
  (Class|KismetSystemLibrary|PauseTimer 0 "MovimentoBasso")
  (Variables|Default|SetVado%20a%20destra? (not (Variables|Default|GetVado%20a%20destra?)))
  (Utilities|Time|SetTimerbyFunctionName 0 "MovimentoAlieno" 0.5 true))

(event EventBeginPlay
  ;[0.15 0.15 0.15 0.5] Camera
  (bind _returnvalue (Actor|GetActorOfClass "/Script/Engine.CameraActor"))
  (Game|Player|SetViewTargetwithBlend (Game|GetPlayerController 0) _returnvalue 0.0 "VTBlend_Linear" 0.0 false)
  ;[0.15 0.15 0.15 0.5] Generazione Alieni
  (for _index (range 0 2)
    (for _index_2 (range 0 5)
      (Game|SpawnActorfromClass "/Game/Blueprints/Alieno.Alieno_C" (Math|Transform|MakeTransform (Variables|Default|GetSpawnRigaAlieni) "0, 0, 0" "1.000000,1.000000,1.000000") "Undefined" "MultiplyWithRoot" 0 0)
      (Variables|Default|SetSpawnRigaAlieni (Math|Vector|MakeVector (.x (Variables|Default|GetSpawnRigaAlieni)) (+ (.y (Variables|Default|GetSpawnRigaAlieni)) 2e+02) (.z (Variables|Default|GetSpawnRigaAlieni)))))
    (Variables|Default|SetSpawnRigaAlieni (Math|Vector|MakeVector (.x (Variables|Default|GetSpawnRigaAlieni)) -7.9e+02 (+ (.z (Variables|Default|GetSpawnRigaAlieni)) -1.5e+02))))
  (Utilities|Time|SetTimerbyFunctionName 0 "MovimentoAlieno" 0.5 true))

(event EventTick
  (params (DeltaSeconds :type Float%20%28single-precision%29)))

(fn ConstructionScript)