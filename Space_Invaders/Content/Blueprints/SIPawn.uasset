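; SIPawn is the player pawn that slides sideways and fires projectiles from its cannon.
; On BeginPlay it adds the ComandiGioco Enhanced Input mapping context to the first local player.
; Laterale input offsets the actor along world Y by a fixed step per trigger, without delta-time scaling.
; Fuoco spawns a Proiettile at the Cannone component, capping live shots at two by counting all Proiettile actors in the world.
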(event Input|EnhancedActionEvents|EnhancedInputActionLaterale
  (params (ActionValue :type Float%20%28double-precision%29) (ElapsedSeconds :type Float%20%28double-precision%29) (TriggeredSeconds :type Float%20%28double-precision%29) (InputAction :type Input%20Action%20Object%20Reference :default "/Game/Input/Laterale.Laterale"))
  (:Triggered
    (Transformation|AddActorWorldOffset (Math|Vector|MakeVector 0.0 (* ActionValue 5.0) 0.0))))

(event Input|EnhancedActionEvents|EnhancedInputActionFuoco
  (params (ActionValue :type Boolean) (ElapsedSeconds :type Float%20%28double-precision%29) (TriggeredSeconds :type Float%20%28double-precision%29) (InputAction :type Input%20Action%20Object%20Reference :default "/Game/Input/Fuoco.Fuoco"))
  (:Started
    (bind _outactors (Actor|GetAllActorsOfClass "/Game/Blueprints/Proiettile.Proiettile_C"))
    (if (not (>= (Utilities|Array|Length _outactors) 2))
      (Game|SpawnActorfromClass "/Game/Blueprints/Proiettile.Proiettile_C" (Math|Transform|MakeTransform (Transformation|GetWorldLocation (Variables|Default|GetCannone)) "0, 0, 0" "1.000000,1.000000,1.000000") "Undefined" "MultiplyWithRoot" 0 0))))

(event EventBeginPlay
  (Input|AddMappingContext (PlayerController|LocalPlayerSubsystems|GetEnhancedInputLocalPlayerSubsystem (Game|GetPlayerController 0)) "/Game/Input/ComandiGioco.ComandiGioco" 0 "(bIgnoreAllPressedKeysUntilRelease=True,bForceImmediately=False,bNotifyUserSettings=False)"))

(fn ConstructionScript)